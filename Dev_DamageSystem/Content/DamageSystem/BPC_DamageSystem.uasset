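; Damage system component that manages an actor's health, healing, blocking and death.
; TakeDamage uses a CanBeDamaged macro to route each damage info struct to block, damage or no damage, based on death, invincibility and blocking state.
; Dispatchers report blocks, deaths and damage responses; non-lethal hits trigger a response and return true only when interruptible or force-interrupting.
; Heal clamps health to the maximum and works only while alive.
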(fn `Heal`
  (params (amountToHeal :type "Float (double-precision)"))
  (returns (newHealth :type "Float (double-precision)"))
  (if (not (`self.isDead`))
    (bind _output_get (set `self.currentHealth` (`KismetMathLibrary.FClamp` (+ (`self.currentHealth`) amountToHeal) 0.0 (`self.maxHealth`))))
    (return _output_get)))

(fn `TakeDamage`
  (params (damageInfo :type "/Game/DamageSystem/S_DamageInfo Structure"))
  (returns (wasDamaged :type Boolean))
  (bind (_damageamount _damagetype _damageresponse _shoulddamageinvincible _canbeblocked _canbeparried _shouldforceinterrupt) (break `/Game/DamageSystem/S_DamageInfo` damageInfo))
  (`self.CanBeDamaged` _shoulddamageinvincible _canbeblocked
    (:`BlockDamage`
      (`self.OnBlocked` _canbeparried)
      (return false))
    (:`DoDamage`
      (bind _output_get (set `self.currentHealth` (- (`self.currentHealth`) _damageamount)))
      (if (<= _output_get 0.0)
        (set `self.isDead` true)
        (`self.OnDeath`)
        (return true)
        (elif (or (`self.isInterruptible`) _shouldforceinterrupt)
          (`self.OnDamageResponse` _damageresponse)
          (return true))))
    (:`NoDamage`
      (return false))))